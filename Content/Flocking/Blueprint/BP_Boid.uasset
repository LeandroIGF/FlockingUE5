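; BP_Boid is a single boid actor for the flocking system, holding a velocity but no steering or movement logic of its own.
; Each tick it can draw a debug arrow along its normalized velocity, gated by DebugVelocityDirection.
; ChangeToLeader marks it as leader by creating a dynamic material instance on its static mesh and tinting the Color parameter red.
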(event EventBeginPlay)

(event Collision|EventActorBeginOverlap
  (params (OtherActor :type Actor%20Object%20Reference)))

(event EventTick
  (params (DeltaSeconds :type Float%20%28single-precision%29))
  (Utilities|FlowControl|Sequence
    (:then_0
      (CallFunction|DrawDebugDirectionArrow))))

(fn ConstructionScript)

(fn DrawDebugDirectionArrow
  (bind _returnvalue (Transformation|GetActorLocation))
  (if (Variables|Default|GetDebugVelocityDirection)
    (Rendering|Debug|DrawDebugArrow _returnvalue (+ _returnvalue (* (Math|Vector|Normalize (Variables|Default|GetVelocity)) 2e+02)) 5.0 "(R=1.000000,G=0.000000,B=0.675047,A=1.000000)" 0.0 5.0)))

(fn ChangetoLeader
  (bind _returnvalue (Rendering|Material|CreateDynamicMaterialInstance (Variables|Default|GetStaticMesh) 0 (Rendering|Material|GetMaterial (Variables|Default|GetStaticMesh) 0) "None" :!class /Script/Engine.PrimitiveComponent))
  (Rendering|Material|SetVectorParameterValue _returnvalue "Color" "(R=1.000000,G=0.017440,B=0.000000,A=1.000000)" :!class /Script/Engine.MaterialInstanceDynamic))