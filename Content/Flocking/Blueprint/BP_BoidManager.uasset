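; BP_BoidManager is a level-placed manager that sets up a flocking simulation when play begins.
; It records its own location as the bounds center and gathers all goal point actors and boids in the level.
; It then picks boids at random, promotes each to a leader and seeds its goal location with its current position.
; Random picks can repeat, so fewer distinct leaders than NumLeaders may result.
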(event EventBeginPlay
  (|CallParentFunction)
  (Variables|Default|SetBoundsCenter (Transformation|GetActorLocation))
  (bind _outactors (Actor|GetAllActorsOfClass "/Game/Flocking/Blueprint/BP_GoalPoint.BP_GoalPoint_C"))
  (Variables|Default|SetGoalActors _outactors)
  (bind _outactors_2 (Actor|GetAllActorsOfClass "/Script/Flocking5_3.Boid"))
  (Variables|Default|SetBoids _outactors_2)
  (for _index (range 0 (- (Variables|Default|GetNumLeaders) 1))
    (Variables|Default|SetBoidRef (.OutItem (Utilities|Array|Random (Variables|Default|GetBoids))))
    (bind _asbp_boid (Utilities|Casting|CastToBP_Boid (Variables|Default|GetBoidRef)))
    (Variables|/Script/Flocking5_3.Boid|SetbLeader _asbp_boid true)
    (Variables|/Script/Flocking5_3.Boid|SetGoalLocation _asbp_boid (Transformation|GetActorLocation (Variables|Default|GetBoidRef)))
    (Default|ChangetoLeader _asbp_boid)))

(event Collision|EventActorBeginOverlap
  (params (OtherActor :type Actor%20Object%20Reference)))

(event EventTick
  (params (DeltaSeconds :type Float%20%28single-precision%29)))

(fn ConstructionScript)